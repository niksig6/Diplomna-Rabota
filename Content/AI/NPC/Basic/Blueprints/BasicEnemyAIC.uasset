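; AI controller for the basic melee enemy that runs its behavior tree and relays attacks to the pawn.
; On BeginPlay it caches the controlled BasicEnemy, starts BasicEnemyBT, stores the player character as target and writes its state to the BasicEnemyState blackboard key.
; AI_Attack changes the state but writes it to a different key, AIState.
; PawnAttack triggers the pawn's basic slash.
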(event Custom|PawnAttack
  (Default|AttackBasicSlash (Variables|Default|GetBasicEnemyPawn)))

(event Custom|AI_Attack
  (bind _output_get (Variables|Default|SetCurrState "NewEnumerator1"))
  (AI|Components|Blackboard|SetValueasEnum (AI|GetBlackboard 0) (Utilities|Name|MakeLiteralName "AIState") _output_get))

(event EventBeginPlay
  (bind _asbasic_enemy (Utilities|Casting|CastToBasicEnemy (Pawn|GetControlledPawn)))
  (Variables|Default|SetBasicEnemyPawn _asbasic_enemy)
  (AI|RunBehaviorTree "/Game/AI/NPC/Basic/Blueprints/BasicEnemyBT.BasicEnemyBT")
  (Variables|Default|SetCurrTarget (Game|GetPlayerCharacter 0))
  (AI|Components|Blackboard|SetValueasEnum (AI|GetBlackboard 0) (Utilities|Name|MakeLiteralName "BasicEnemyState") (Variables|Default|GetCurrState)))

(fn ConstructionScript)