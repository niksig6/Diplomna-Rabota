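; FightDirector coordinates enemy attacks in a level and detects when every enemy in its list is dead.
; Each enemy gets a random priority grade; a looping timer rescales grades by enemy facing against camera direction, favouring opposed vectors.
; The top-graded enemy's AI controller then attacks, and its grade is re-rolled.
; Tick counts dead enemies to move Mansion 1 on to Mansion2; optional debug widgets can display grades.
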(event Custom|AttackTrigger
  ;[1 1 1] Debug for the attack priority of enemy characters
  (CallFunction|RecalculateScores)
  (bind _loc_highestgradedai1 (CallFunction|FindHighestGrade))
  (bind _asbasic_enemy_aic (Utilities|Casting|CastToBasicEnemyAIC (AI|GetAIController _loc_highestgradedai1)))
  (Default|AIAttack _asbasic_enemy_aic)
  (Utilities|Map|Add (Variables|Default|GetEnemyGrading) _loc_highestgradedai1 (Math|Random|RandomFloatinRange 1.0 5.0)))

(event EventTick
  (params (DeltaSeconds :type Float%20%28single-precision%29))
  (bind _enemylist (Variables|Default|GetEnemyList))
  (Utilities|FlowControl|Delay 0.2)
  (for _array_element _enemylist
    (Variables|Default|SetEnemyCount (Utilities|Array|Length _enemylist))
    (if (Variables|/Game/AI/NPC/Basic/Blueprints/BasicEnemy.BasicEnemy_C|GetisDead _array_element)
      (bind _result (Math|Integer|IncrementInt (Variables|Default|GetDeadEnemies))
        (:%20%20
          (Variables|Default|SetDeadEnemies _result)
          (Development|PrintString (Utilities|String|ToString(Integer) (Variables|Default|GetDeadEnemies)))))))
  (if (== (Variables|Default|GetDeadEnemies) (Variables|Default|GetEnemyCount))
    (bind _returnvalue (Game|GetCurrentLevelName true))
    (switch string _returnvalue
      (:Mansion1
        (Development|PrintString "Level completed! Switching to level 2 ...")
        (Utilities|FlowControl|Delay 5.0)
        (Game|OpenLevel(byName) "Mansion2")))
    (else
      (Variables|Default|SetDeadEnemies 0)
      (Variables|Default|SetEnemyCount 0))))

(event EventBeginPlay
  ;[1 1 1] Debug for the attack priority of enemy characters
  (for _array_element (Variables|Default|GetEnemyList)
    ;;[1 1 1] Switch with AddDebugWidgets for debug
    (CallFunction|AddAttackHierarchy _array_element))
  (Utilities|Time|SetTimerbyEvent (delegate Custom|AttackTrigger) 3.0 true))

(fn ConstructionScript)

(fn FindHighestGrade
  (bind _keys (Utilities|Map|Keys (Variables|Default|GetEnemyGrading)))
  (for _array_element _keys
    (if (> (.Value (Utilities|Map|Find (Variables|Default|GetEnemyGrading) _array_element)) (LocalVariables|GetLoc_HighestValue))
      (LocalVariables|SetLoc_HighestValue (.Value (Utilities|Map|Find (Variables|Default|GetEnemyGrading) _array_element)))
      (LocalVariables|SetLoc_HighestGradedAI _array_element)))
  (return (LocalVariables|GetLoc_HighestValue) (LocalVariables|GetLoc_HighestGradedAI)))

(fn AddDebugWidgets
  (params (EnemyInstance :type Basic%20Enemy%20Object%20Reference%20%28by%20ref%29))
  (Utilities|Map|Add (Variables|Default|GetEnemyGrading) EnemyInstance (Math|Random|RandomFloatinRange 1.0 5.0))
  (bind _returnvalue (UserInterface|CreateWidget "/Game/AI/NPC/Basic/Blueprints/DebugBasicAI.DebugBasicAI_C" 0 EnemyInstance (.Value (Utilities|Map|Find (Variables|Default|GetEnemyGrading) EnemyInstance))))
  (bind _output_get (LocalVariables|SetLoc_Widget _returnvalue))
  (Utilities|Map|Add (Variables|Default|GetEnemyWidgets) EnemyInstance _output_get)
  (bind _returnvalue_2 (AddComponent|AddWidgetComponent EnemyInstance false))
  (UserInterface|SetWidget _returnvalue_2 (LocalVariables|GetLoc_Widget)))

(fn UpdateDebugWidgets
  (params (%20EnemyInstance :type Basic%20Enemy%20Object%20Reference))
  (if (Variables|Default|GetHasDebugWidget)
    (Variables|/Game/AI/NPC/Basic/Blueprints/DebugBasicAI.DebugBasicAI_C|SetFightingGrade (.Value (Utilities|Map|Find (Variables|Default|GetEnemyWidgets) %20EnemyInstance)) (.Value (Utilities|Map|Find (Variables|Default|GetEnemyGrading) %20EnemyInstance)))))

(fn RecalculateScores
  (CallFunction|ScorebyPostition))

(fn ScorebyPostition
  (bind _enemygrading (Variables|Default|GetEnemyGrading))
  (for _array_element (Variables|Default|GetEnemyList)
    (Development|PrintString (Utilities|String|ToString(Float) (* (Math|Vector|DotProduct (Transformation|GetActorForwardVector _array_element) (Math|Vector|GetForwardVector (Camera|GetCameraRotation (Game|GetPlayerCameraManager 0)))) -1.0)))
    (Utilities|Map|Add _enemygrading _array_element (* (.Value (Utilities|Map|Find _enemygrading _array_element)) (+ (Math|Float|NormalizetoRange (* (Math|Vector|DotProduct (Transformation|GetActorForwardVector _array_element) (Math|Vector|GetForwardVector (Camera|GetCameraRotation (Game|GetPlayerCameraManager 0)))) -1.0) -1.0 1.0) 0.5)))
    (CallFunction|UpdateDebugWidgets _array_element)))

(fn AddAttackHierarchy
  (params (EnemyInstance :type Basic%20Enemy%20Object%20Reference))
  (Utilities|Map|Add (Variables|Default|GetEnemyGrading) EnemyInstance (Math|Random|RandomFloatinRange 1.0 5.0)))