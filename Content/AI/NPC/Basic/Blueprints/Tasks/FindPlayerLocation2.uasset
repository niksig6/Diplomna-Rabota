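; Behavior tree task for basic NPCs that writes the player character's current location to a Blackboard target key.
; It line traces on the Camera channel from the NPC to the player, focusing the AI controller on the player when nothing blocks it and clearing focus otherwise.
; It then sets the NPC's max walk speed to a configurable value and finishes successfully.
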(event EventReceiveExecuteAI
  (params (OwnerController :type AI%20Controller%20Object%20Reference) (ControlledPawn :type Pawn%20Object%20Reference))
  (Variables|Default|SetOwner%20Controller OwnerController)
  (Variables|Default|SetControlled%20Pawn ControlledPawn)
  (AI|BehaviorTree|SetBlackboardValueasVector (Variables|Default|GetBB_TargetLocation) (Transformation|GetActorLocation (Game|GetPlayerCharacter 0)))
  (CallFunction|SetFocus)
  (CallFunction|SetWalkSpeed)
  (AI|BehaviorTree|FinishExecute true))

(fn SetFocus
  (bind _controlled_pawn (Variables|Default|GetControlled%20Pawn))
  (bind _owner_controller (Variables|Default|GetOwner%20Controller))
  (bind _outhit (Collision|LineTraceByChannel (Transformation|GetActorLocation _controlled_pawn) (Transformation|GetActorLocation (Game|GetPlayerCharacter 0)) "TraceTypeQuery2" false (Utilities|Array|MakeArray _controlled_pawn) "None"))
  (if (== (.hitactor _outhit) (Game|GetPlayerCharacter 0))
    (AI|SetFocus _owner_controller (.hitactor _outhit))
    (else
      (AI|ClearFocus _owner_controller))))

(fn SetWalkSpeed
  (bind _ascharacter (Utilities|Casting|CastToCharacter (Variables|Default|GetControlled%20Pawn)))
  (Variables|/Script/Engine.CharacterMovementComponent|SetMaxWalkSpeed (Variables|/Script/Engine.Character|GetCharacterMovement _ascharacter) (Variables|Default|GetWalkSpeed))
  (return))